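; TestPC is a player controller that lets the player request a respawn when it has no pawn.
; The Respawn input action prints a message if a pawn is still possessed, and otherwise calls RequestRespawn.
; RequestRespawn casts the game mode to GameMode_Default and passes the controller to its Respawn function, which handles the respawn itself.
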(event EventBeginPlay)

(event EventTick
  (params (DeltaSeconds :type Float%20%28single-precision%29)))

(fn ConstructionScript)

(event Custom|RequestRespawn
  (bind _returnvalue (Game|GetGameMode))
  (Utilities|IsValid _returnvalue
    (:Is%20Valid
      (bind _asgame_mode_default (Utilities|Casting|CastToGameMode_Default _returnvalue))
      (Utilities|IsValid _asgame_mode_default
        (:Is%20Valid
          (bind _returnvalue_2 (Utilities|Casting|CastToPlayerController self))
          (Default|Respawn _asgame_mode_default _returnvalue_2))))))

(event Input|ActionEvents|InputActionRespawn
  (params (Key :type Key%20Structure :default "AnyKey"))
  (:Pressed
    (Utilities|IsValid (Pawn|GetControlledPawn self)
      (:Is%20Valid
        (Development|PrintString "Controller is still in possession of a pawn"))
      (:Is%20Not%20Valid
        (CallFunction|RequestRespawn)))))