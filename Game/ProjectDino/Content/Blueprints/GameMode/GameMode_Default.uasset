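; Default game mode that handles respawning players as Cubeasaurus characters.
; On BeginPlay it caches the first Camera_Main actor found in the level.
; Respawn spawns and possesses a new Cubeasaurus, then spawns a Test weapon, attaches it to the character and stores it as its Weapon.
; It then notifies the camera of the respawn and prints the weapon's instigator controller name.
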(event Custom|Respawn
  (params (Player%20Controller :type Player%20Controller%20Object%20Reference))
  (bind _camera_reference (Variables|Default|GetCamera%20Reference))
  (Utilities|IsValid Player%20Controller
    (:Is%20Valid
      (bind _returnvalue (Game|SpawnActorfromClass "/Game/Blueprints/Character/Cubeasaurus.Cubeasaurus_C" (Math|Transform|MakeTransform "0, 0, 0" "0, 0, 0" "1,1,1") "AlwaysSpawn" 0 0)) ; Respawn the player's character
      (Utilities|IsValid _returnvalue
        (:Is%20Valid
          (Pawn|Possess Player%20Controller _returnvalue)
          (bind _returnvalue_2 (Game|SpawnActorfromClass "/Game/Blueprints/Weapons/Test.Test_C" (Math|Transform|MakeTransform "0, 0, 0" "0, 0, 0" "1,1,1") "AlwaysSpawn" 0 0)) ; Respawn the player's weapon
          (Class|Actor|AttachRootComponenttoActor _returnvalue_2 _returnvalue "None" "SnapToTarget" true) ; Attach the weapon to the character
          (bind _output_get (Variables|/Game/Blueprints/Character/Cubeasaurus.Cubeasaurus_C|SetWeapon _returnvalue _returnvalue_2))
          (Utilities|IsValid _camera_reference
            (:Is%20Valid
              (Default|PlayerRespawned _camera_reference)
              (Development|PrintString (Utilities|GetDisplayName (Game|GetInstigatorController _output_get))))))))))

(event EventBeginPlay
  (bind _outactors (Actor|GetAllActorsOfClass "/Game/Blueprints/Camera/Camera_Main.Camera_Main_C"))
  (Variables|Default|SetCamera%20Reference (Utilities|Array|Get(acopy) _outactors)))

(event EventTick
  (params (DeltaSeconds :type Float%20%28single-precision%29)))

(fn ConstructionScript)