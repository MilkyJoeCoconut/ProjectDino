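; Player character Cubeasaurus, with control-yaw-relative movement, an aimed turret weapon, its own HUD and a PlayerIndex for controller lookup.
; Both aim axes share one path that shifts an absolute-location Sphere target and yaws the Test weapon toward it, setting the angle Shoot fires along.
; Hit drains Health, then destroys pawn and weapon and asks TestPC to respawn.
; F and right shoulder are debug damage keys that skip weapon cleanup and respawn.
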(event EventActorBeginOverlap
  (params (OtherActor :type Actor%20Object%20Reference)))

(event EventTick
  (params (DeltaSeconds :type Float%20%28single-precision%29)))

(event EventBeginPlay
  (bind _asgame_mode_default (Utilities|Casting|CastToGameMode_Default (Game|GetGameMode)))
  (Variables|Default|SetCamera%20Reference (Variables|/Game/Blueprints/GameMode/GameMode_Default.GameMode_Default_C|GetCamera%20Reference _asgame_mode_default))
  (Variables|/Script/Engine.SceneComponent|SetbAbsoluteLocation (Variables|Default|GetSphere) true)
  (bind _returnvalue (UserInterface|CreateWidget "/Game/Blueprints/UserInterface/HUD.HUD_C"))
  (bind _output_get (Variables|UserInterface|SetHUD%20Reference _returnvalue))
  (UserInterface|Viewport|AddtoViewport _output_get 0)
  (Input|SetInputModeGameOnly (Game|GetPlayerController (Variables|UserInterface|GetPlayer%20Index)))
  (Development|PrintString (Utilities|String|ToString(Integer) (Variables|UserInterface|GetPlayer%20Index))))

(event Input|ActionEvents|InputActionShoot
  (params (Key :type Key%20Structure :default "AnyKey"))
  (:Pressed
    (bind _astest (Utilities|Casting|CastToTest (Variables|Movement/Aim|GetWeapon)))
    (Default|Shoot _astest (Variables|Movement/Aim|GetTarget_Rot))))

(event Input|KeyboardEvents|F
  (params (Key :type Key%20Structure :default "AnyKey"))
  ;[1 1 1] HUD Health Test
  (:Pressed
    (Variables|UserInterface|SetHealth (- (Variables|UserInterface|GetHealth) 0.25))
    (if (<= (Variables|UserInterface|GetHealth) 0.0)
      (Actor|DestroyActor))))

(event Input|GamepadEvents|GamepadRightShoulder
  (params (Key :type Key%20Structure :default "AnyKey"))
  ;[1 1 1] HUD Health Test
  (:Pressed
    (Variables|UserInterface|SetHealth (- (Variables|UserInterface|GetHealth) 0.25))
    (if (<= (Variables|UserInterface|GetHealth) 0.0)
      (Actor|DestroyActor))))

(fn ConstructionScript)

(fn Hit
  (bind _output_get (Variables|UserInterface|SetHealth (- (Variables|UserInterface|GetHealth) 0.25)))
  (if (<= _output_get 0.0)
    (Class|Pawn|DetachfromControllerPendingDestroy)
    (Actor|DestroyActor)
    (bind _astest (Utilities|Casting|CastToTest (Variables|Movement/Aim|GetWeapon)))
    (Actor|DestroyActor _astest)
    (bind _astest_pc (Utilities|Casting|CastToTestPC (Game|GetPlayerController (Variables|UserInterface|GetPlayer%20Index))))
    (Default|Respawn _astest_pc)))

(event Input|AxisEvents|InputAxisMoveX
  (params (AxisValue :type Float%20%28single-precision%29))
  (Pawn|Input|AddMovementInput (Math|Vector|GetForwardVector (Math|Rotator|MakeRotator 0.0 0.0 (.Yaw (Math|Rotator|BreakRotator (Pawn|GetControlRotation :!class /Script/Engine.Pawn))))) AxisValue false)
  (Variables|Movement/Aim|SetF_Move AxisValue))

(event Input|AxisEvents|InputAxisMoveY
  (params (AxisValue :type Float%20%28single-precision%29))
  (Pawn|Input|AddMovementInput (Math|Vector|GetRightVector (Math|Rotator|MakeRotator 0.0 0.0 (.Yaw (Math|Rotator|BreakRotator (Pawn|GetControlRotation :!class /Script/Engine.Pawn))))) AxisValue false)
  (Variables|Movement/Aim|SetR_Move AxisValue))

(event Input|AxisEvents|InputAxisAimX
  (params (AxisValue :type Float%20%28single-precision%29))
  (bind _sphere (Variables|Default|GetSphere))
  (bind _returnvalue (Transformation|GetWorldLocation _sphere))
  (bind _returnvalue_2 (Transformation|GetWorldLocation _sphere))
  (Transformation|SetWorldLocation _sphere (Math|Vector|MakeVector (+ (.x (Math|Vector|MakeVector (* AxisValue 2.0) (* (stale Input|AxisEvents|InputAxisAimY AxisValue) 2.0) 0.0)) (.x _returnvalue)) (+ (.y (Math|Vector|MakeVector (* AxisValue 2.0) (* (stale Input|AxisEvents|InputAxisAimY AxisValue) 2.0) 0.0)) (.y _returnvalue)) (+ (.z (Math|Vector|MakeVector (* AxisValue 2.0) (* (stale Input|AxisEvents|InputAxisAimY AxisValue) 2.0) 0.0)) (.z _returnvalue))) false false)
  (bind _output_get (Variables|Movement/Aim|SetTarget_Rot (.yaw (Math|Rotator|FindLookatRotation (Transformation|GetWorldLocation (Variables|Character|GetMesh)) (Math|Vector|MakeVector (.x _returnvalue_2) (.y _returnvalue_2) 0.0)))))
  (bind _astest (Utilities|Casting|CastToTest (Variables|Movement/Aim|GetWeapon)))
  (Transformation|SetWorldRotation (Variables|/Game/Blueprints/Weapons/Test.Test_C|GetStaticMesh _astest) (Math|Rotator|MakeRotator 0.0 0.0 _output_get) false false))

(event Input|AxisEvents|InputAxisAimY
  (params (AxisValue :type Float%20%28single-precision%29))
  (bind _sphere (Variables|Default|GetSphere))
  (bind _returnvalue (Transformation|GetWorldLocation _sphere))
  (bind _returnvalue_2 (Transformation|GetWorldLocation _sphere))
  (Transformation|SetWorldLocation _sphere (Math|Vector|MakeVector (+ (.x (Math|Vector|MakeVector (* (stale Input|AxisEvents|InputAxisAimX AxisValue) 2.0) (* AxisValue 2.0) 0.0)) (.x _returnvalue)) (+ (.y (Math|Vector|MakeVector (* (stale Input|AxisEvents|InputAxisAimX AxisValue) 2.0) (* AxisValue 2.0) 0.0)) (.y _returnvalue)) (+ (.z (Math|Vector|MakeVector (* (stale Input|AxisEvents|InputAxisAimX AxisValue) 2.0) (* AxisValue 2.0) 0.0)) (.z _returnvalue))) false false)
  (bind _output_get (Variables|Movement/Aim|SetTarget_Rot (.yaw (Math|Rotator|FindLookatRotation (Transformation|GetWorldLocation (Variables|Character|GetMesh)) (Math|Vector|MakeVector (.x _returnvalue_2) (.y _returnvalue_2) 0.0)))))
  (bind _astest (Utilities|Casting|CastToTest (Variables|Movement/Aim|GetWeapon)))
  (Transformation|SetWorldRotation (Variables|/Game/Blueprints/Weapons/Test.Test_C|GetStaticMesh _astest) (Math|Rotator|MakeRotator 0.0 0.0 _output_get) false false))