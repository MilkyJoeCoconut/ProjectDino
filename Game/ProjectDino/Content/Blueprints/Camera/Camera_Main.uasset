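; Shared spring-arm camera that keeps two local players' Cubeasaurus characters in view.
; On begin play or respawn, it becomes both controllers' view target and caches the characters; on death it jumps to origin.
; Tick eases it toward the center of the players' minimum-area rectangle, with speed scaled by the focus point's distance from origin.
; Player separation sets the clamped arm length, zooming out as they spread.
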(event Custom|Player%20Died
  (Transformation|SetActorLocation "0, 0, 0" false false))

(event Custom|Player%20Respawned
  (Game|Player|SetViewTargetwithBlend (Game|GetPlayerController 0) self 0.0 "VTBlend_Linear" 0.0 false)
  (Utilities|Array|Clear (Variables|PlayerReferences|GetPlayers))
  (bind _outactors (Actor|GetAllActorsOfClass "/Game/Blueprints/Character/Cubeasaurus.Cubeasaurus_C"))
  (for _index (range 0 1)
    (Utilities|IsValid (Utilities|Array|Get(acopy) _outactors _index)
      (:Is%20Valid
        (Utilities|Array|AddUnique (Variables|PlayerReferences|GetPlayers) (Utilities|Array|Get(acopy) _outactors _index))))))

(event EventBeginPlay
  (Game|Player|SetViewTargetwithBlend (Game|GetPlayerController 0) self 0.0 "VTBlend_Linear" 0.0 false)
  (Utilities|Array|Clear (Variables|PlayerReferences|GetPlayers))
  (bind _outactors (Actor|GetAllActorsOfClass "/Game/Blueprints/Character/Cubeasaurus.Cubeasaurus_C"))
  (for _index (range 0 1)
    (Utilities|IsValid (Utilities|Array|Get(acopy) _outactors _index)
      (:Is%20Valid
        (Utilities|Array|AddUnique (Variables|PlayerReferences|GetPlayers) (Utilities|Array|Get(acopy) _outactors _index))))))

(event EventActorBeginOverlap
  (params (OtherActor :type Actor%20Object%20Reference)))

(event EventTick
  (params (DeltaSeconds :type Float%20%28single-precision%29)))

(event EventTick
  (params (DeltaSeconds :type Float%20%28single-precision%29))
  (bind _player_locations (Variables|PlayerReferences|GetPlayer%20Locations))
  (bind _player_locations_2 (Variables|PlayerReferences|GetPlayer%20Locations))
  (Utilities|Array|Clear (Variables|PlayerReferences|GetPlayer%20Locations))
  (for _array_element (Variables|PlayerReferences|GetPlayers)
    (Utilities|IsValid _array_element
      (:Is%20Valid
        (Utilities|Array|AddUnique (Variables|PlayerReferences|GetPlayer%20Locations) (Transformation|GetActorLocation _array_element)))))
  (for (_ _array_index) _player_locations_2
    (if (>= (- _array_index 1) 0)
      (Variables|PlayerReferences|SetMax%20Distance (Math|Float|Absolute(Float) (Math|Vector|VectorLength (- (Utilities|Array|Get(acopy) _player_locations _array_index) (Utilities|Array|Get(acopy) _player_locations (- _array_index 1))))))))
  (bind _outrectcenter (Class|KismetMathLibrary|MinimumAreaRectangle _player_locations_2 (Transformation|GetActorLocation) false))
  (Variables|CameraReferences|SetTarget%20Position _outrectcenter)
  (bind _output_get (Variables|CameraReferences|SetCamera%20Focus (Math|Interpolation|VInterpTo (Variables|CameraReferences|GetCurrent%20Position) (Variables|CameraReferences|GetTarget%20Position) (Utilities|Time|GetWorldDeltaSeconds) (Variables|CameraReferences|GetInterp%20Speed))))
  (Transformation|SetActorLocation _output_get false false)
  (Variables|CameraReferences|SetCurrent%20Position (Transformation|GetActorLocation))
  (Variables|/Script/Engine.SpringArmComponent|SetTargetArmLength (Variables|Default|GetSpringArm) (Math|Float|Clamp(Float) (Variables|PlayerReferences|GetMax%20Distance) 7e+02 2e+03))
  (Variables|CameraReferences|SetInterp%20Speed (/ (Math|Vector|VectorLength (Variables|CameraReferences|GetCamera%20Focus)) 1.5e+02)))

(fn ConstructionScript)

(fn UpdateCameraVector
  (bind _players (Variables|PlayerReferences|GetPlayers))
  (Variables|CameraReferences|SetTarget%20Position (/ (+ (Transformation|GetActorLocation (Utilities|Array|Get(acopy) _players)) (Transformation|GetActorLocation (Utilities|Array|Get(acopy) _players 1))) 2)))